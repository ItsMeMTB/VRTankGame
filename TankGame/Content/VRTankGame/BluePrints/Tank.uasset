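; Player-driven Renault FT-17 tank for the VR tank game, with movement, turret and gun controlled by input axes.
; MoveForward offsets the actor along local X, and MoveRight rotates it on both pitch and yaw.
; LookRight and LookUp rotate the turret and gun components around their local pitch axes.
; Each axis value is scaled by its own speed variable, without delta-time scaling.
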(event `InputAxis|MoveForward`
  (params (AxisValue :type "Float (single-precision)"))
  ;[1 1 1] Forward
  (`self.K2_AddActorLocalOffset` (`KismetMathLibrary.MakeVector` (* AxisValue (`self.Speed`)))))

(event `InputAxis|MoveRight`
  (params (AxisValue :type "Float (single-precision)"))
  (bind _returnvalue (* AxisValue (`self.SpeedRotation`)))
  ;[1 1 1] Right
  (`self.K2_AddActorLocalRotation` (`KismetMathLibrary.MakeRotator` 0.0 _returnvalue _returnvalue)))

(event `InputAxis|LookRight`
  (params (AxisValue :type "Float (single-precision)"))
  ;[1 1 1] Turret
  (`SceneComponent.K2_AddLocalRotation` (`self.Tank_Renault_FT_17_v15_Turret_0`) (`KismetMathLibrary.MakeRotator` 0.0 (* AxisValue (`self.Turret`))) false false))

(event `InputAxis|LookUp`
  (params (AxisValue :type "Float (single-precision)"))
  ;[1 1 1] Gun
  (`SceneComponent.K2_AddLocalRotation` (`self.Tank_Renault_FT_17_v15_Gun_9`) (`KismetMathLibrary.MakeRotator` 0.0 (* AxisValue (`self.Gun`))) false false))

(fn `UserConstructionScript`)